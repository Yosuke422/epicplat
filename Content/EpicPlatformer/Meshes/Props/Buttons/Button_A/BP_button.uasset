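; BP_button is a pressure button that opens a linked Gate while pressed by a ball or character.
; Box overlap by BP_Ball or CharacterBP opens the Gate, swaps the button material and plays the PRESS timeline, lerping the push mesh between A and B.
; Any end overlap, without actor filtering, closes the Gate, restores the material and reverses the timeline.
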(event OnComponentBeginOverlap(Box)
  (params (OverlappedComponent :type Primitive%20Component%20Object%20Reference) (OtherActor :type Actor%20Object%20Reference) (OtherComp :type Primitive%20Component%20Object%20Reference) (OtherBodyIndex :type Integer) (bFromSweep :type Boolean) (SweepResult :type Hit%20Result%20Structure%20%28by%20ref%29))
  (Utilities|FlowControl|Sequence
    (:then_0
      (Utilities|Casting|CastToBP_Ball OtherActor))
    (:then_1
      (Utilities|Casting|CastToCharacterBP OtherActor)))
  (Utilities|FlowControl|Sequence
    (:then_0
      (Default|Open (Variables|Default|GetGate)))
    (:then_1
      (Rendering|Material|SetMaterial (Variables|Default|GetSM_Button_A_Push) 0 "/Game/EpicPlatformer/Meshes/Props/Buttons/Button_A/Material/M_Button_A_2.M_Button_A_2"))
    (:then_2
      (bind _movement (Timeline|PRESS Play)
        (:Update
          (Transformation|SetRelativeLocation (Variables|Default|GetSM_Button_A_Push) (Math|Vector|Lerp(Vector) (Variables|Default|GetA) (Variables|Default|GetB) _movement) false false))))))

(event OnComponentEndOverlap(Box)
  (params (OverlappedComponent :type Primitive%20Component%20Object%20Reference) (OtherActor :type Actor%20Object%20Reference) (OtherComp :type Primitive%20Component%20Object%20Reference) (OtherBodyIndex :type Integer))
  (Utilities|FlowControl|Sequence
    (:then_0
      (Default|Close (Variables|Default|GetGate)))
    (:then_1
      (Rendering|Material|SetMaterial (Variables|Default|GetSM_Button_A_Push) 0 "/Game/EpicPlatformer/Meshes/Props/Buttons/Button_A/Material/M_Button_A_1.M_Button_A_1"))
    (:then_2
      (bind _movement (Timeline|PRESS Reverse)
        (:Update
          (Transformation|SetRelativeLocation (Variables|Default|GetSM_Button_A_Push) (Math|Vector|Lerp(Vector) (Variables|Default|GetA) (Variables|Default|GetB) _movement) false false))))))

(fn ConstructionScript)